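; Magazine pickup Blueprint whose look reflects the magazine's rarity: Common, Rare, Master or Legendary.
; UpdateMagazinePickupMaterial switches on MagazineRarity to set the pickup mesh material and the Sparkle effect's color and beam height, which grows with rarity from zero at Common.
; The graph holds only this visual update and does not call it; BeginPlay, overlap, Tick and the construction script are empty.
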(event `self.UpdateMagazinePickupMaterial`
  (bind _sparkle (`self.Sparkle`))
  (bind _sparkle_2 (`self.Sparkle`))
  (bind _sparkle_3 (`self.Sparkle`))
  (bind _sparkle_4 (`self.Sparkle`))
  (switch `ERarity` (`self.MagazineRarity`)
    (:`Common`
      (`PrimitiveComponent.SetMaterial` (`self.PickupMesh`) 0 "/Game/Materials/RarityMaterial/CommonMaterial.CommonMaterial")
      (`FXSystemComponent.SetColorParameter` _sparkle_3 "RarityColor" (`self.Common`))
      (`FXSystemComponent.SetFloatParameter` _sparkle_3 "BeamHeight" 0.0))
    (:`Rare`
      (`PrimitiveComponent.SetMaterial` (`self.PickupMesh`) 0 "/Game/Materials/RarityMaterial/RareMaterial.RareMaterial")
      (`FXSystemComponent.SetColorParameter` _sparkle_4 "RarityColor" (`self.Rare`))
      (`FXSystemComponent.SetFloatParameter` _sparkle_4 "BeamHeight" 1.0))
    (:`Master`
      (`PrimitiveComponent.SetMaterial` (`self.PickupMesh`) 0 "/Game/Materials/PickupMaterials/MasterMaterial.MasterMaterial")
      (`FXSystemComponent.SetColorParameter` _sparkle "RarityColor" (`self.Master`))
      (`FXSystemComponent.SetFloatParameter` _sparkle "BeamHeight" 1.5))
    (:`Legendary`
      (`PrimitiveComponent.SetMaterial` (`self.PickupMesh`) 0 "/Game/Materials/RarityMaterial/LegendaryMaterial.LegendaryMaterial")
      (`FXSystemComponent.SetColorParameter` _sparkle_2 "RarityColor" (`self.Legendary`))
      (`FXSystemComponent.SetFloatParameter` _sparkle_2 "BeamHeight" 2.5))))

(fn `UserConstructionScript`)